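; Learning Agents training environment that scores, ends and resets episodes for BP_Agent, which appears to learn lap driving on a track.
; Reward fires on checkpoint hits, shrinking with steps since the previous one; the reward pass also clears the flag, counts steps and accumulates the total.
; Episodes terminate at a step limit or completed lap, and reset delegates to the agent.
; Off-track penalty and termination nodes exist but are unconnected.
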(fn GatherAgentCompletion
  (params (AgentId :type Integer))
  (bind _returnvalue (Class|LearningAgentsManagerListener|GetAgent AgentId "/Game/_Project/Agent/BP_Agent.BP_Agent_C"))
  (return (Class|LearningAgentsCompletions|Completionor (Class|LearningAgentsCompletions|MakeCompletiononCondition (== (Variables|/Game/_Project/Agent/BP_Agent.BP_Agent_C|GetStepCount _returnvalue) 10000) "Termination" "ConditionCompletion" false 0) (Class|LearningAgentsCompletions|MakeCompletiononCondition (>= (Variables|/Game/_Project/Agent/BP_Agent.BP_Agent_C|GetLap _returnvalue) 1) "Termination" "ConditionCompletion" false 0) "Running")))

(fn GatherAgentReward
  (params (AgentId :type Integer))
  (Variables|Default|SetRewardActor (Class|LearningAgentsManagerListener|GetAgent AgentId "/Game/_Project/Agent/BP_Agent.BP_Agent_C"))
  (LocalVariables|SetTempOutReward (+ 0.0 (Class|LearningAgentsRewards|MakeRewardonCondition (Variables|/Game/_Project/Agent/BP_Agent.BP_Agent_C|GetCheckointHit (Variables|Default|GetRewardActor)) (- 2.0 (/ (- (Math|Conversions|ToFloat(Integer) (Variables|/Game/_Project/Agent/BP_Agent.BP_Agent_C|GetStepCount (Variables|Default|GetRewardActor))) (Math|Conversions|ToFloat(Integer) (Variables|/Game/_Project/Agent/BP_Agent.BP_Agent_C|GetPreviousStepCount (Variables|Default|GetRewardActor)))) 1e+04)) "BadCollisionReward" false 0) 0.0))
  (Utilities|FlowControl|Sequence
    (:then_0
      (if (Variables|/Game/_Project/Agent/BP_Agent.BP_Agent_C|GetCheckointHit (Variables|Default|GetRewardActor))
        (Variables|/Game/_Project/Agent/BP_Agent.BP_Agent_C|SetCheckointHit (Variables|Default|GetRewardActor) false)
        (Variables|/Game/_Project/Agent/BP_Agent.BP_Agent_C|SetPreviousStepCount (Variables|Default|GetRewardActor) (Variables|/Game/_Project/Agent/BP_Agent.BP_Agent_C|GetStepCount (Variables|Default|GetRewardActor)))))
    (:then_1
      (Variables|/Game/_Project/Agent/BP_Agent.BP_Agent_C|SetStepCount (Variables|Default|GetRewardActor) (+ (Variables|/Game/_Project/Agent/BP_Agent.BP_Agent_C|GetStepCount (Variables|Default|GetRewardActor)) 1)))
    (:then_2
      (Variables|/Game/_Project/Agent/BP_Agent.BP_Agent_C|SetCummulativeReward (Variables|Default|GetRewardActor) (+ (LocalVariables|GetTempOutReward) (Variables|/Game/_Project/Agent/BP_Agent.BP_Agent_C|GetCummulativeReward (Variables|Default|GetRewardActor))))
      (return (LocalVariables|GetTempOutReward)))))

(fn ResetAgentEpisode
  (params (AgentId :type Integer))
  (Default|ResetAgent (Class|LearningAgentsManagerListener|GetAgent AgentId "/Game/_Project/Agent/BP_Agent.BP_Agent_C")))