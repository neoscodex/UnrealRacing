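; Learning Agents interactor that lets BP_Agent actors perceive and drive through a checkpoint course with road and ground surfaces.
; Observations form a fixed-size float array of checkpoint direction and distance, yaw sine and cosine, velocity direction, and on/off-track state.
; Each trace hit adds direction, normalized distance and Ground/Road tag flags, zero-padded on misses.
; Three three-way discrete actions map through a lookup array into agent rotation and movement.
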(fn SpecifyAgentObservation
  (params (InObservationSchema :type Learning%20Agents%20Observation%20Schema%20Object%20Reference))
  (return (Class|LearningAgentsObservations|SpecifyStaticArrayObservation InObservationSchema (Class|LearningAgentsObservations|SpecifyFloatObservation InObservationSchema 1.0) (Variables|Default|GetArraySize))))

(fn SpecifyAgentAction
  (params (InActionSchema :type Learning%20Agents%20Action%20Schema%20Object%20Reference))
  (return (Class|LearningAgentsActions|SpecifyStructAction InActionSchema (Utilities|Map|MakeMap "Vertical" (Class|LearningAgentsActions|SpecifyExclusiveDiscreteAction InActionSchema 3) "Horizontal" (Class|LearningAgentsActions|SpecifyExclusiveDiscreteAction InActionSchema 3) "Rotate" (Class|LearningAgentsActions|SpecifyExclusiveDiscreteAction InActionSchema 3)))))

(fn GatherAgentObservation
  (params (InObservationObject :type Learning%20Agents%20Observation%20Object%20Object%20Reference) (AgentId :type Integer))
  (Variables|Default|SetObsActor (Class|LearningAgentsManagerListener|GetAgent AgentId "/Game/_Project/Agent/BP_Agent.BP_Agent_C"))
  (Utilities|Array|Clear (Variables|Default|GetObservationsArray))
  (Utilities|Array|AppendArray (Variables|Default|GetObservationsArray) (Utilities|Array|MakeArray (Class|LearningAgentsObservations|MakeFloatObservation InObservationObject (.x (Math|Vector|Normalize (- (Transformation|GetActorLocation (Utilities|Array|Get(acopy) (Variables|/Game/_Project/Agent/BP_Agent.BP_Agent_C|GetCheckpointArray (Variables|Default|GetObsActor)) (Variables|/Game/_Project/Agent/BP_Agent.BP_Agent_C|GetCurrentCheckpointIndex (Variables|Default|GetObsActor)))) (Transformation|GetActorLocation (Variables|Default|GetObsActor))))) "FloatObservation" false 0) (Class|LearningAgentsObservations|MakeFloatObservation InObservationObject (.y (Math|Vector|Normalize (- (Transformation|GetActorLocation (Utilities|Array|Get(acopy) (Variables|/Game/_Project/Agent/BP_Agent.BP_Agent_C|GetCheckpointArray (Variables|Default|GetObsActor)) (Variables|/Game/_Project/Agent/BP_Agent.BP_Agent_C|GetCurrentCheckpointIndex (Variables|Default|GetObsActor)))) (Transformation|GetActorLocation (Variables|Default|GetObsActor))))) "FloatObservation" false 0) (Class|LearningAgentsObservations|MakeFloatObservation InObservationObject (Math|Float|Clamp(Float) (/ (Math|Vector|Distance(Vector) (Transformation|GetActorLocation (Utilities|Array|Get(acopy) (Variables|/Game/_Project/Agent/BP_Agent.BP_Agent_C|GetCheckpointArray (Variables|Default|GetObsActor)) (Variables|/Game/_Project/Agent/BP_Agent.BP_Agent_C|GetCurrentCheckpointIndex (Variables|Default|GetObsActor)))) (Transformation|GetActorLocation (Variables|Default|GetObsActor))) (Variables|/Game/_Project/Agent/BP_Agent.BP_Agent_C|GetMaxDistance (Variables|Default|GetObsActor))) -1.0) "FloatObservation" false 0) (Class|LearningAgentsObservations|MakeFloatObservation InObservationObject (Math|Trig|Sin(Degrees) (.yaw (Transformation|GetWorldRotation (Variables|/Game/_Project/Agent/BP_Agent.BP_Agent_C|GetScene (Variables|Default|GetObsActor))))) "FloatObservation" false 0) (Class|LearningAgentsObservations|MakeFloatObservation InObservationObject (Math|Trig|Cos(Degrees) (.yaw (Transformation|GetWorldRotation (Variables|/Game/_Project/Agent/BP_Agent.BP_Agent_C|GetScene (Variables|Default|GetObsActor))))) "FloatObservation" false 0) (Class|LearningAgentsObservations|MakeFloatObservation InObservationObject (.x (Math|Vector|Normalize (Transformation|GetVelocity (Variables|Default|GetObsActor)))) "FloatObservation" false 0) (Class|LearningAgentsObservations|MakeFloatObservation InObservationObject (.y (Math|Vector|Normalize (Transformation|GetVelocity (Variables|Default|GetObsActor)))) "FloatObservation" false 0)))
  (Utilities|Array|AppendArray (Variables|Default|GetObservationsArray) (Utilities|Array|MakeArray (Class|LearningAgentsObservations|MakeFloatObservation InObservationObject (Math|Conversions|ToFloat(Boolean) (Variables|/Game/_Project/Agent/BP_Agent.BP_Agent_C|GetOffTrack (Variables|Default|GetObsActor))) "FloatObservation" false 0) (Class|LearningAgentsObservations|MakeFloatObservation InObservationObject (Math|Conversions|ToFloat(Boolean) (Variables|/Game/_Project/Agent/BP_Agent.BP_Agent_C|GetOnTrack (Variables|Default|GetObsActor))) "FloatObservation" false 0)))
  (for _array_element (Variables|/Game/_Project/Agent/BP_Agent.BP_Agent_C|GetHitArray (Variables|Default|GetObsActor))
    (if (.bBlockingHit (Collision|BreakHitResult _array_element))
      (Utilities|Array|AppendArray (Variables|Default|GetObservationsArray) (Utilities|Array|MakeArray (Class|LearningAgentsObservations|MakeFloatObservation InObservationObject (.x (Math|Vector|Normalize (- (.Location (Collision|BreakHitResult _array_element)) (Transformation|GetActorLocation (Variables|Default|GetObsActor))))) "FloatObservation" false 0) (Class|LearningAgentsObservations|MakeFloatObservation InObservationObject (.y (Math|Vector|Normalize (- (.Location (Collision|BreakHitResult _array_element)) (Transformation|GetActorLocation (Variables|Default|GetObsActor))))) "FloatObservation" false 0) (Class|LearningAgentsObservations|MakeFloatObservation InObservationObject (Math|Float|Clamp(Float) (/ (.Distance (Collision|BreakHitResult _array_element)) (Variables|/Game/_Project/Agent/BP_Agent.BP_Agent_C|GetMaxDistance (Variables|Default|GetObsActor))) -1.0) "FloatObservation" false 0) (Class|LearningAgentsObservations|MakeFloatObservation InObservationObject (Math|Conversions|ToFloat(Boolean) (Actor|ActorHasTag (.HitActor (Collision|BreakHitResult _array_element)) "Ground")) "FloatObservation" false 0) (Class|LearningAgentsObservations|MakeFloatObservation InObservationObject (Math|Conversions|ToFloat(Boolean) (Actor|ActorHasTag (.HitActor (Collision|BreakHitResult _array_element)) "Road")) "FloatObservation" false 0)))
      (else
        (Utilities|Array|AppendArray (Variables|Default|GetObservationsArray) (Utilities|Array|MakeArray (Class|LearningAgentsObservations|MakeFloatObservation InObservationObject 0.0 "FloatObservation" false 0) (Class|LearningAgentsObservations|MakeFloatObservation InObservationObject 0.0 "FloatObservation" false 0) (Class|LearningAgentsObservations|MakeFloatObservation InObservationObject 0.0 "FloatObservation" false 0) (Class|LearningAgentsObservations|MakeFloatObservation InObservationObject 0.0 "FloatObservation" false 0) (Class|LearningAgentsObservations|MakeFloatObservation InObservationObject 0.0 "FloatObservation" false 0))))))
  (return (Class|LearningAgentsObservations|MakeStaticArrayObservation InObservationObject (Variables|Default|GetObservationsArray))))

(fn PerformAgentAction
  (params (InActionObject :type Learning%20Agents%20Action%20Object%20Object%20Reference) (InActionObjectElement :type Learning%20Agents%20Action%20Object%20Element%20Structure%20%28by%20ref%29) (AgentId :type Integer))
  (Variables|Default|SetActActor (Class|LearningAgentsManagerListener|GetAgent AgentId "/Game/_Project/Agent/BP_Agent.BP_Agent_C"))
  (bind _outelements (Class|LearningAgentsActions|GetStructAction InActionObject InActionObjectElement))
  (Utilities|FlowControl|Sequence
    (:then_0
      (bind _outindex (Class|LearningAgentsActions|GetExclusiveDiscreteAction InActionObject (.Value (Utilities|Map|Find _outelements "Rotate")) "DiscreteExclusiveAction" false 0))
      (Default|RotateActor (Variables|Default|GetActActor) (Utilities|Array|Get(acopy) (LocalVariables|GetVectorFloats) _outindex)))
    (:then_1
      (bind _outindex_2 (Class|LearningAgentsActions|GetExclusiveDiscreteAction InActionObject (.Value (Utilities|Map|Find _outelements "Vertical")) "DiscreteExclusiveAction" false 0))
      (bind _outindex_3 (Class|LearningAgentsActions|GetExclusiveDiscreteAction InActionObject (.Value (Utilities|Map|Find _outelements "Horizontal")) "DiscreteExclusiveAction" false 0))
      (Default|MoveActor (Variables|Default|GetActActor) (Utilities|Array|Get(acopy) (LocalVariables|GetVectorFloats) _outindex_2) (Utilities|Array|Get(acopy) (LocalVariables|GetVectorFloats) _outindex_3)))))