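; Racing agent that registers with a Learning Agents manager and moves by physics forces and yaw rotation.
; Enhanced Input drives it only in heuristic mode.
; Each tick it casts line traces into HitArray, while overlaps with ordered checkpoints track progress and laps and hits on Ground-tagged actors flag off-track.
; ResetAgent returns it to PlayerStart, appends step count, checkpoints passed and cumulative reward to a CSV log, then clears episode state.
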(event Input|EnhancedActionEvents|EnhancedInputActionIA_Move
  (params (ActionValue :type Vector%202D%20Structure) (ElapsedSeconds :type Float%20%28double-precision%29) (TriggeredSeconds :type Float%20%28double-precision%29) (InputAction :type Input%20Action%20Object%20Reference :default "/Game/_Project/Input/IA_Move.IA_Move"))
  ;[0.15 0.15 0.15 0.5] Move Agent
  (if (Variables|Default|GetIsHeuristic)
    (CallFunction|MoveActor (.x ActionValue) (.y ActionValue))))

(event Input|EnhancedActionEvents|EnhancedInputActionIA_Look
  (params (ActionValue :type Float%20%28double-precision%29) (ElapsedSeconds :type Float%20%28double-precision%29) (TriggeredSeconds :type Float%20%28double-precision%29) (InputAction :type Input%20Action%20Object%20Reference :default "/Game/_Project/Input/IA_Look.IA_Look"))
  ;[0.15 0.15 0.15 0.5] Rotate Agent
  (if (Variables|Default|GetIsHeuristic)
    (CallFunction|RotateActor ActionValue)))

(event Collision|EventHit
  (params (MyComp :type Primitive%20Component%20Object%20Reference) (Other :type Actor%20Object%20Reference) (OtherComp :type Primitive%20Component%20Object%20Reference) (bSelfMoved :type Boolean) (HitLocation :type Vector :default "0, 0, 0") (HitNormal :type Vector :default "0, 0, 0") (NormalImpulse :type Vector :default "0, 0, 0") (Hit :type Hit%20Result%20Structure%20%28by%20ref%29))
  (Variables|Default|SetOffTrack (Actor|ActorHasTag Other "Ground")))

(event Collision|EventActorBeginOverlap
  (params (OtherActor :type Actor%20Object%20Reference))
  ;[0.15 0.15 0.15 0.5] Update CurrentCheckpointIndex on overlap with next Checkpoint, Update NumberOfCheckpoitsPassed, Update CheckpointHit
  (if (== OtherActor (Utilities|Array|Get(acopy) (Variables|Default|GetCheckpointArray) (Variables|Default|GetCurrentCheckpointIndex)))
    (Utilities|FlowControl|Sequence
      (:then_0
        (if (!= (+ (Variables|Default|GetCurrentCheckpointIndex) 1) (Utilities|Array|Length (Variables|Default|GetCheckpointArray)))
          (Variables|Default|SetCurrentCheckpointIndex (+ (Variables|Default|GetCurrentCheckpointIndex) 1))
          (else
            (Variables|Default|SetCurrentCheckpointIndex 0)
            (Variables|Default|SetLap (+ (Variables|Default|GetLap) 1)))))
      (:then_1
        (Variables|Default|SetNumberOfCheckpointsPassed (+ (Variables|Default|GetNumberOfCheckpointsPassed) 1))
        (Variables|Default|SetCheckointHit true)))))

(event EventBeginPlay
  (|CallParentFunction)
  (Utilities|FlowControl|Sequence
    (:then_0
      ;[0.15 0.15 0.15 0.502] Register Agent with Manager
      (bind _outactors (Actor|GetAllActorswithTag "LearningAgentsManager"))
      (for _array_element _outactors
        (Utilities|IsValid (Actor|GetComponentbyClass _array_element "/Script/LearningAgents.LearningAgentsManager")
          (:Is%20Valid
            (Class|LearningAgentsManager|AddAgent (Actor|GetComponentbyClass _array_element "/Script/LearningAgents.LearningAgentsManager") self))
          (:Is%20Not%20Valid
            (Development|PrintString "Could not find Learning Agents manager. Did we forget to add one to the scene?")))))
    (:then_1
      (bind _asplayer_controller (Utilities|Casting|CastToPlayerController (Pawn|GetController))
        (:then
          _)
        (:CastFailed
          (Utilities|IsValid (PlayerController|LocalPlayerSubsystems|GetEnhancedInputLocalPlayerSubsystem _asplayer_controller)
            (:Is%20Valid
              _))))
      (Input|AddMappingContext (PlayerController|LocalPlayerSubsystems|GetEnhancedInputLocalPlayerSubsystem _asplayer_controller) "/Game/_Project/Input/IMC_Agent.IMC_Agent" 0 "(bIgnoreAllPressedKeysUntilRelease=True,bForceImmediately=False,bNotifyUserSettings=False)"))
    (:then_2
      ;[0.15 0.15 0.15 0.502] Assign CheckpointArray and Set CurrentCheckpointIndex
      (bind _outactors_2 (Actor|GetAllActorsOfClass "/Game/_Project/Other/BP_CheckpointArray.BP_CheckpointArray_C"))
      (Variables|Default|SetCheckpointArray (Variables|/Game/_Project/Other/BP_CheckpointArray.BP_CheckpointArray_C|GetCheckpointArray (Utilities|Array|Get(acopy) _outactors_2)))
      (Variables|Default|SetCurrentCheckpointIndex 0)
      (Variables|Default|SetLap 0))
    (:then_3
      (bind _outactors_3 (Actor|GetAllActorsOfClass "BP_Agent_C"))
      (Variables|Default|SetActors%20to%20Ignore _outactors_3))
    (:then_4
      ;[0.15 0.15 0.15 0.5] Set start rotation
      (CallFunction|RotateActor (.yaw (Variables|/Script/Engine.SceneComponent|GetRelativeRotation (Variables|Default|GetAgent))))
      (CallFunction|CreateCSVFile))))

(event EventTick
  (params (DeltaSeconds :type Float%20%28single-precision%29))
  (bind _temphitarray (Variables|Default|GetTempHitArray))
  ;[0.15 0.15 0.15 0.5] Cast RayTraces and assign Arrays
  (Utilities|FlowControl|Sequence
    (:then_0
      (for (_array_element _array_index) (Variables|Default|GetTraceArray)
        (bind _hit (CallFunction|CastTrace _array_element))
        (Utilities|Array|SetArrayElem _temphitarray _array_index _hit))
      (Variables|Default|SetHitArray _temphitarray))))

(fn ConstructionScript)

(fn ResetAgent
  (bind _returnvalue (Actor|GetActorOfClass "/Script/Engine.PlayerStart"))
  (Transformation|SetActorLocation (Transformation|GetActorLocation _returnvalue) false false)
  (Transformation|SetActorRotation (Transformation|GetActorRotation _returnvalue))
  (Transformation|SetRelativeRotation (Variables|Default|GetScene) (Transformation|GetActorRotation _returnvalue) false false)
  (Class|PrimitiveComponent|SetAllPhysicsLinearVelocity (Variables|Default|GetAgent) "0, 0, 0" false)
  (CallFunction|LogData)
  (Variables|Default|SetStepCount 0)
  (Variables|Default|SetPreviousStepCount 0)
  (Variables|Default|SetCurrentCheckpointIndex 0)
  (Variables|Default|SetNumberOfCheckpointsPassed 0)
  (Variables|Default|SetLap 0)
  (Variables|Default|SetCummulativeReward 0.0)
  (Variables|Default|SetOffTrack false))

(fn CastTrace
  (params (Trace :type Vector))
  (bind _agent (Variables|Default|GetAgent))
  (bind _relativelocation (Variables|/Script/Engine.SceneComponent|GetRelativeLocation _agent))
  (bind _outhit (Collision|LineTraceByChannel _relativelocation (+ _relativelocation (Math|Vector|RotateVector (* (Math|Vector|Normalize Trace) (Variables|Default|GetMaxDistance)) (Variables|/Script/Engine.SceneComponent|GetRelativeRotation (Variables|Default|GetScene)))) "TraceTypeQuery1" false (Variables|Default|GetActors%20to%20Ignore) "ForOneFrame" true "(R=1.000000,G=0.000000,B=0.000000,A=1.000000)" "(R=0.000000,G=1.000000,B=0.000000,A=1.000000)" 0.01))
  (return _outhit))

(fn MoveActor
  (params (Y :type Float%20%28double-precision%29) (X :type Float%20%28double-precision%29))
  (LocalVariables|SetMoveVector (Math|Vector2D|Normalize2D (Math|Vector2D|MakeVector2D X Y)))
  (if (> X 0.0)
    (LocalVariables|SetMoveVector (Math|Vector2D|MakeVector2D (* (.x (LocalVariables|GetMoveVector)) 1.5) (.y (LocalVariables|GetMoveVector)))))
  (Physics|AddForce (Variables|Default|GetAgent) (Math|Vector|RotateVector (Math|Conversions|ToVector(Vector2D) (* (LocalVariables|GetMoveVector) (Variables|Default|GetVelocity))) (Variables|/Script/Engine.SceneComponent|GetRelativeRotation (Variables|Default|GetScene))) "None" false))

(fn RotateActor
  (params (RotationAmount :type Float%20%28double-precision%29))
  (Transformation|SetRelativeRotation (Variables|Default|GetScene) (Math|Rotator|MakeRotator 0.0 0.0 (+ RotationAmount (.yaw (Variables|/Script/Engine.SceneComponent|GetRelativeRotation (Variables|Default|GetScene))))) false false))

(fn LogData
  (bind _filename (Variables|Default|GetFileName))
  (bind _returnvalue (Utilities|String|Append _filename "_unreal_racing_data.csv"))
  (bind _returnvalue_2 (Utilities|String|Append "C:\\Projects\\Unreal\\Logs\\Racing\\" _returnvalue))
  (bind _returnvalue_3 (Class|BlueprintFileUtilsBPLibrary|FileExists _returnvalue_2))
  (if _returnvalue_3
    (Class|FileSDKBPLibrary|WriteStringtoFile _returnvalue_2 (Utilities|String|Append (Utilities|String|ToString(Integer) (Variables|Default|GetStepCount)) "," (Utilities|String|ToString(Integer) (Variables|Default|GetNumberOfCheckpointsPassed)) "," (Utilities|String|ToString(Float) (Variables|Default|GetCummulativeReward)) " 
") true "AutoDetect")))

(fn CreateCSVFile
  (bind _filename (Variables|Default|GetFileName))
  (bind _returnvalue (Utilities|String|Append _filename "_unreal_racing_data.csv"))
  (bind _returnvalue_2 (Utilities|String|Append "C:\\Projects\\Unreal\\Logs\\Racing\\" _returnvalue))
  (bind _returnvalue_3 (Class|BlueprintFileUtilsBPLibrary|FileExists _returnvalue_2))
  (if _returnvalue_3
    (Development|PrintString "File already exists.")
    (else
      (Class|FileSDKBPLibrary|CreateFile _returnvalue_2 true true)
      (Class|FileSDKBPLibrary|WriteStringtoFile _returnvalue_2 (Utilities|String|Append "StepCount" "," "NumberOfCheckpointsPassed" "," "CummulativeReward" " 
") false "AutoDetect"))))